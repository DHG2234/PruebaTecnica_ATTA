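; BP_Area is a damageable hazard zone that applies damage over time to the player inside its collision sphere.
; Overlap begin and end resolve the player through PlayerRefMessage, toggle its inside-area flag, start or stop its DOT functions, and play an enter/exit HUD notification.
; AnyDamage reduces the area's health, but checks for depletion before subtracting, so the area is destroyed on the hit after health reaches zero.
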(event OnComponentBeginOverlap(SphereCollision)
  (params (OverlappedComponent :type Primitive%20Component%20Object%20Reference) (OtherActor :type Actor%20Object%20Reference) (OtherComp :type Primitive%20Component%20Object%20Reference) (OtherBodyIndex :type Integer) (bFromSweep :type Boolean) (SweepResult :type Hit%20Result%20Structure%20%28by%20ref%29))
  ;[0.8782 0.4333 1] Start/End DOT to Player
  (Utilities|StartDOTtoPlayer OtherActor))

(event OnComponentEndOverlap(SphereCollision)
  (params (OverlappedComponent :type Primitive%20Component%20Object%20Reference) (OtherActor :type Actor%20Object%20Reference) (OtherComp :type Primitive%20Component%20Object%20Reference) (OtherBodyIndex :type Integer))
  ;[0.8782 0.4333 1] Start/End DOT to Player
  (Utilities|EndDOTtoPlayer OtherActor))

(event EventBeginPlay)

(event EventTick
  (params (DeltaSeconds :type Float%20%28single-precision%29)))

(event Game|Damage|EventAnyDamage
  (params (Damage :type Float%20%28single-precision%29) (DamageType :type Damage%20Type%20Object%20Reference) (InstigatedBy :type Controller%20Object%20Reference) (DamageCauser :type Actor%20Object%20Reference))
  (Variables|Default|SetAreaDmgReceived Damage)
  (if (<= (Variables|Health|GetArea_CurrentHealth) 0.0)
    (Actor|DestroyActor)
    (else
      (CallFunction|AreaTakeDamage))))

(fn ConstructionScript)

(fn AreaTakeDamage
  (bind _output_get (Variables|Health|SetArea_CurrentHealth (- (Variables|Health|GetArea_CurrentHealth) (Variables|Default|GetAreaDmgReceived))))
  (if (<= _output_get 0.0)
    _))

(fn AreaRef
  (return self))

(fn PlayerRef
  (return 0))